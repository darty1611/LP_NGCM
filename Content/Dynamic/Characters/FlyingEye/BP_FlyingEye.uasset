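; Flying eye enemy character with animation-driven hurt, attack and death events.
; Each event plays an override animation on the AnimationComponent's instance, and Attack calls SpawnProjectile once its animation completes.
; Death clears default-group overrides and plays in a separate Death slot.
; Whether that animation completes or is cancelled, it spawns a health orb, notifies MyLP_NGCMGameMode of the kill and destroys the actor.
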(event `self.HurtAnim`
  (`PaperZDAnimInstance.K2_PlayAnimationOverride` (`PaperZDAnimationComponent.AnimInstance` (`self.AnimationComponent`)) "/Game/Stacic/Characters/FlyingEye/Animations/AnimSequences/Hurt.Hurt" "DefaultSlot" 1.0 0.0))

(event `self.DieAnim`
  (bind _animinstance (`PaperZDAnimationComponent.AnimInstance` (`self.AnimationComponent`)))
  (`PaperZDAnimInstance.StopAnimationOverrideByGroup` _animinstance "DefaultGroup")
  (`PaperZDPlaySlotOverrideAction.PlayAnimationOverrideWithCallbacks` _animinstance "/Game/Stacic/Characters/FlyingEye/Animations/AnimSequences/Death.Death" "Death"
    (:`OnCompleted`
      _)
    (:`OnCancelled`
      _))
  (`|SpawnActorFromClass` "/Game/Dynamic/Items/HealthOrb/BP_HealthOrb.BP_HealthOrb_C" (`self.GetTransform`) "Undefined" "MultiplyWithRoot" null null)
  (bind _asmy_lp_ngcmgame_mode (cast `/Game/Dynamic/GameModes/MyLP_NGCMGameMode` (`GameplayStatics.GetGameMode`))
    (:`then`
      (`/Game/Dynamic/GameModes/MyLP_NGCMGameMode.EnemyDeathNotify` _asmy_lp_ngcmgame_mode))
    (:`CastFailed`
      _))
  (`self.K2_DestroyActor`))

(event `self.Attack`
  (`PaperZDPlaySlotOverrideAction.PlayAnimationOverrideWithCallbacks` (`PaperZDAnimationComponent.AnimInstance` (`self.AnimationComponent`)) "/Game/Stacic/Characters/FlyingEye/Animations/AnimSequences/Attack.Attack"
    (:`OnCompleted`
      (`self.spawnProjectile`))))

(fn `UserConstructionScript`)