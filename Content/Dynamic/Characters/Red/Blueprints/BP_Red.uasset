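; BP_Red is the Red character Blueprint, handling jump animation, melee attack and bow shooting through what appears to be a PaperZD AnimInstance.
; Jumping or walking off a ledge sends the Locomotion state machine to airborne.
; Attack and Shoot play override animations gated by a shared IsAnimationPlaying flag, with Shoot spawning an arrow on completion or cancellation.
; AttackBox overlap only prints a debug string, with no damage logic.
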(event `self.ReceiveBeginPlay`)

(event `self.ReceiveTick`
  (params (DeltaSeconds :type "Float (single-precision)")))

(event `self.OnJumped`
  (`PaperZDAnimInstance.JumpToNode` (`PaperZDAnimationComponent.AnimInstance` (`self.AnimationComponent`)) "airborne" "Locomotion" :!label _label))

(event `self.OnWalkingOffLedge`
  (params (PreviousFloorImpactNormal :type "Vector Structure (by ref)") (PreviousFloorContactNormal :type "Vector Structure (by ref)") (PreviousLocation :type "Vector Structure (by ref)") (TimeDelta :type "Float (single-precision)"))
  (goto _label))

(event `self.Attack`
  ;[1 1 1] Attacking
  (if (not (`self.isAnimationPlaying`))
    (`PaperZDPlaySlotOverrideAction.PlayAnimationOverrideWithCallbacks` (`PaperZDAnimationComponent.AnimInstance` (`self.AnimationComponent`)) "/Game/Stacic/Characters/Red/Animations/AnimSequences/Attack.Attack"
      (:`then`
        (set `self.isAnimationPlaying` true))
      (:`OnCompleted`
        (set `self.isAnimationPlaying` false :!label _label_2))
      (:`OnCancelled`
        (goto _label_2)))))

(event `self.attackBox.OnComponentBeginOverlap`
  (params (OverlappedComponent :type "PrimitiveComponent Object Reference") (OtherActor :type "Actor Object Reference") (OtherComp :type "PrimitiveComponent Object Reference") (OtherBodyIndex :type Integer) (bFromSweep :type Boolean) (SweepResult :type "HitResult Structure (by ref)"))
  ;[1 1 1] Attacking
  (`KismetSystemLibrary.PrintString` "Hello"))

(event `self.Shoot`
  ;[1 1 1] Shooting
  (if (not (`self.isAnimationPlaying`))
    (`PaperZDPlaySlotOverrideAction.PlayAnimationOverrideWithCallbacks` (`PaperZDAnimationComponent.AnimInstance` (`self.AnimationComponent`)) "/Game/Stacic/Characters/Red/Animations/AnimSequences/Bow.Bow"
      (:`then`
        (set `self.isAnimationPlaying` true))
      (:`OnCompleted`
        (set `self.isAnimationPlaying` false :!label _label_3)
        (`self.spawnArrow`))
      (:`OnCancelled`
        (goto _label_3)))))

(fn `UserConstructionScript`)