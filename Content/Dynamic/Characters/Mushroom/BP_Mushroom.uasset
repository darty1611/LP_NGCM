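; BP_Mushroom is a Mushroom enemy character Blueprint that handles its hurt, attack and death animations.
; HurtAnim, Attack and DieAnim events play PaperZD-style animation overrides through the AnimationComponent's AnimInstance.
; DieAnim stops default-group overrides, plays Dead in the Death slot, waits on the returned duration, notifies MyLP_NGCMGameMode of the enemy death, then destroys the actor.
; Attack's trailing delay leads to no further logic.
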(event `self.HurtAnim`
  (`PaperZDAnimInstance.K2_PlayAnimationOverride` (`PaperZDAnimationComponent.AnimInstance` (`self.AnimationComponent`)) null "DefaultSlot" 1.0 0.0))

(event `self.DieAnim`
  (bind _animinstance (`PaperZDAnimationComponent.AnimInstance` (`self.AnimationComponent`)))
  (`PaperZDAnimInstance.StopAnimationOverrideByGroup` _animinstance "DefaultGroup")
  (bind _animationlength (`PaperZDAnimInstance.K2_PlayAnimationOverride` _animinstance "/Game/Stacic/Characters/AxeSkeleton/Animations/AnimSequences/Dead.Dead" "Death" 1.0 0.0))
  (`KismetSystemLibrary.Delay` _animationlength)
  (bind _asmy_lp_ngcmgame_mode (cast `/Game/Dynamic/GameModes/MyLP_NGCMGameMode` (`GameplayStatics.GetGameMode`))
    (:`then`
      (`/Game/Dynamic/GameModes/MyLP_NGCMGameMode.EnemyDeathNotify` _asmy_lp_ngcmgame_mode))
    (:`CastFailed`
      _))
  (`self.K2_DestroyActor`))

(event `self.Attack`
  (bind _animationlength (`PaperZDAnimInstance.K2_PlayAnimationOverride` (`PaperZDAnimationComponent.AnimInstance` (`self.AnimationComponent`)) "/Game/Stacic/Characters/Mushroom/Animations/AnimSequences/Attack.Attack" "DefaultSlot" 1.0 0.0))
  (`KismetSystemLibrary.Delay` _animationlength))

(fn `UserConstructionScript`)