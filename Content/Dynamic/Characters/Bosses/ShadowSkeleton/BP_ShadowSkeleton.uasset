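; Shadow Skeleton boss Blueprint that plays the boss's action and death animations.
; Events for spawning axe skeletons, shooting a soul and attacking each play an animation override on the AnimationComponent's AnimInstance.
; The death event stops all overrides, plays Death in its own slot, waits for the returned duration, then destroys the actor.
; The gameplay effects of these actions are not implemented in this graph.
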(event `self.ReceiveBeginPlay`)

(event `self.spawnAxeSkeletonsAnim`
  (`PaperZDPlaySlotOverrideAction.PlayAnimationOverrideWithCallbacks` (`PaperZDAnimationComponent.AnimInstance` (`self.AnimationComponent`)) "/Game/Stacic/Characters/Bosses/ShadowSkeleton/Animations/AnimSequences/SpawnSkeletons.SpawnSkeletons"))

(event `self.shootSoulAnim`
  (`PaperZDAnimInstance.K2_PlayAnimationOverride` (`PaperZDAnimationComponent.AnimInstance` (`self.AnimationComponent`)) "/Game/Stacic/Characters/Bosses/ShadowSkeleton/Animations/AnimSequences/ShootSoul.ShootSoul" "DefaultSlot" 1.0 0.0))

(event `self.Attack`
  (`PaperZDAnimInstance.K2_PlayAnimationOverride` (`PaperZDAnimationComponent.AnimInstance` (`self.AnimationComponent`)) "/Game/Stacic/Characters/Bosses/ShadowSkeleton/Animations/AnimSequences/Attack.Attack" "DefaultSlot" 1.0 0.0))

(event `self.DieAnim`
  (bind _animinstance (`PaperZDAnimationComponent.AnimInstance` (`self.AnimationComponent`)))
  (`PaperZDAnimInstance.StopAllAnimationOverrides` _animinstance)
  (bind _animationlength (`PaperZDAnimInstance.K2_PlayAnimationOverride` _animinstance "/Game/Stacic/Characters/Bosses/ShadowSkeleton/Animations/AnimSequences/Death.Death" "Death" 1.0 0.0))
  (`KismetSystemLibrary.Delay` _animationlength)
  (`self.K2_DestroyActor`))

(fn `UserConstructionScript`)