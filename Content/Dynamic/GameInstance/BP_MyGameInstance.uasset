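; Game instance that owns the player's save data, keeping a BP_MyGameSave object available for the whole session.
; On Init it synchronously loads the save slot, or creates a fresh save object if none exists.
; SavePlayer copies a player data struct into that object and writes it to disk, either synchronously or asynchronously.
; ClearSave deletes the slot and reloads to a blank save, while GetSaveData exposes the current object.
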(event `self.ReceiveInit`
  (`/Game/Dynamic/SaveGame/BPI_SaveGame.LoadSaveData` false))

(event `/Game/Dynamic/SaveGame/BPI_SaveGame.SaveSaveData`
  (params (Async :type Boolean))
  ;[1 1 1] Save Game
  (if Async
    (`AsyncActionHandleSaveGame.AsyncSaveGameToSlot` (`self.Save Data`) (`self.Save Slot Name`))
    (else
      (`KismetSystemLibrary.PrintString` "salvou")
      (`GameplayStatics.SaveGameToSlot` (`self.Save Data`) (`self.Save Slot Name`)))))

(event `/Game/Dynamic/SaveGame/BPI_SaveGame.LoadSaveData`
  (params (Async :type Boolean))
  (bind _save_slot_name (`self.Save Slot Name`))
  ;[1 1 1] Load Game
  (bind _returnvalue (`GameplayStatics.DoesSaveGameExist` (`self.Save Slot Name`)))
  (if _returnvalue
    (if Async
      (bind _savegame (`AsyncActionHandleSaveGame.AsyncLoadGameFromSlot` _save_slot_name)
        (:`Completed`
          (bind _asbp_my_game_save (cast `/Game/Dynamic/SaveGame/BP_MyGameSave` _savegame))
          (set `self.Save Data` _asbp_my_game_save)))
      (else
        (bind _returnvalue_2 (`GameplayStatics.LoadGameFromSlot` _save_slot_name))
        (bind _asbp_my_game_save_2 (cast `/Game/Dynamic/SaveGame/BP_MyGameSave` _returnvalue_2))
        (set `self.Save Data` _asbp_my_game_save_2)))
    (else
      (bind _returnvalue_3 (`GameplayStatics.CreateSaveGameObject` "/Game/Dynamic/SaveGame/BP_MyGameSave.BP_MyGameSave_C"))
      (set `self.Save Data` _returnvalue_3))))

(event `/Game/Dynamic/SaveGame/BPI_SaveGame.SavePlayer`
  (params (`Player Save` :type "/Game/Dynamic/SaveGame/S_SaveData Structure") (Async :type Boolean))
  (set `/Game/Dynamic/SaveGame/BP_MyGameSave.Save Data Structure` `Player Save` (`self.Save Data`))
  (`/Game/Dynamic/SaveGame/BPI_SaveGame.SaveSaveData` Async))

(event `/Game/Dynamic/SaveGame/BPI_SaveGame.ClearSave`
  (bind _returnvalue (`GameplayStatics.DeleteGameInSlot` (`self.Save Slot Name`)))
  (if _returnvalue
    (`/Game/Dynamic/SaveGame/BPI_SaveGame.LoadSaveData` false)))

(fn `GetSaveData`
  (returns (SaveData :type "/Game/Dynamic/SaveGame/BP_MyGameSave Object Reference"))
  (return (`self.Save Data`)))